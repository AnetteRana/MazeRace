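; BP_PlayerParent is the parent player Blueprint for a maze race, handling goal and collision rules.
; It caches its spawn location on BeginPlay.
; Overlapping an actor of exactly the BP_Goal class calls SwitchLevel on BP_MazeRaceGameModeBase.
; Any other overlap moves the player back to the cached start without sweeping.
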(event Collision|EventActorBeginOverlap
  (params (OtherActor :type Actor%20Object%20Reference))
  ;[1 1 1] collisions
  (if (== (Utilities|GetClass OtherActor) "/Game/Blueprints/BP_Goal.BP_Goal_C")
    ;[1 1 1] collide with goal = new level
    (bind _asbp_maze_race_game_mode_base (Utilities|Casting|CastToBP_MazeRaceGameModeBase (Game|GetGameMode)))
    (Default|SwitchLevel _asbp_maze_race_game_mode_base)
    (else
      ;[1 1 1] collide with other = back to start
      (Transformation|SetActorLocation (Variables|Default|GetmyStartLocation) false false))))

(event EventBeginPlay
  ;[1 1 1] set start location
  (Variables|Default|SetmyStartLocation (Transformation|GetActorLocation)))

(fn ConstructionScript)