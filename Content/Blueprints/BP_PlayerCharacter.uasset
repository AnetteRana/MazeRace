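; Player character for a maze race that resets to its start location on overlapping anything other than the goal.
; Tick moves it by vertical and horizontal values scaled by Speed, using unswept SetActorLocation with Z pinned to zero.
; Overlapping BP_Goal calls SwitchLevel on the maze race game mode.
; On possession, ColorSelect sets the cube's material from PlayerInt, giving four player colors with gray as fallback.
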(event EventBeginPlay)

(event Collision|EventActorBeginOverlap
  (params (OtherActor :type Actor%20Object%20Reference))
  ;[1 1 1] collisions
  (if (== (Utilities|GetClass OtherActor) "/Game/Blueprints/BP_Goal.BP_Goal_C")
    (Development|PrintString "NEXT LEVEL")
    (bind _asbp_maze_race_game_mode_base (Utilities|Casting|CastToBP_MazeRaceGameModeBase (Game|GetGameMode)))
    (Default|SwitchLevel _asbp_maze_race_game_mode_base)
    (else
      (Transformation|SetActorLocation (Variables|Default|GetmyStartLocation) false false))))

(event EventTick
  (params (DeltaSeconds :type Float%20%28single-precision%29))
  (bind _returnvalue (Transformation|GetActorLocation))
  (bind (_x _y) (Math|Vector|BreakVector _returnvalue))
  ;[1 1 1] movement
  (Transformation|SetActorLocation (Math|Vector|MakeVector (+ (* (Variables|Default|Getspeed) (Input|AxisValues|Getvertical)) _x) (+ _y (* (Variables|Default|Getspeed) (Input|AxisValues|Gethorizontal))) 0.0) false false))

(event EventPossessed
  (params (NewController :type Controller%20Object%20Reference))
  (CallFunction|ColorSelect)
  ;[1 1 1] print text for testing
  (Development|PrintString (Utilities|String|Append (Utilities|String|Append (Utilities|String|Append "Possessed: " (Utilities|GetDisplayName NewController)) "   /   ") (Utilities|String|ToString(Integer) (Variables|Default|GetplayerInt)))))

(fn ConstructionScript
  (Variables|Default|Setspeed 1e+01))

(fn ColorSelect
  (switch int (Variables|Default|GetplayerInt)
    (:Default
      (Rendering|Material|SetMaterial (Variables|Default|GetCube) 0 "/Game/Materials/MAT_Gray.MAT_Gray"))
    (:0
      (Rendering|Material|SetMaterial (Variables|Default|GetCube) 0 "/Game/Materials/MAT_Red.MAT_Red"))
    (:1
      (Rendering|Material|SetMaterial (Variables|Default|GetCube) 0 "/Game/Materials/MAT_Green.MAT_Green"))
    (:2
      (Rendering|Material|SetMaterial (Variables|Default|GetCube) 0 "/Game/Materials/MAT_Blue.MAT_Blue"))
    (:3
      (Rendering|Material|SetMaterial (Variables|Default|GetCube) 0 "/Game/Materials/MAT_Yellow.MAT_Yellow"))))