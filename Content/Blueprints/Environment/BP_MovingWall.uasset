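; BP_MovingWall is an environment actor, a wall that slides back and forth along one horizontal axis.
; The construction script caches the actor's placed location as the start point.
; Each Tick sets the location to that start plus a sine of game time scaled by Speed and Distance, on X or Y according to the XAxis flag, without sweeping.
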(event EventTick
  (params (DeltaSeconds :type Float%20%28single-precision%29))
  (bind _startlocation (Variables|Default|GetStartLocation))
  (bind _startlocation_2 (Variables|Default|GetStartLocation))
  (bind (_x _y _z) (Math|Vector|BreakVector _startlocation_2))
  (bind (_x_2 _y_2 _z_2) (Math|Vector|BreakVector _startlocation))
  (if (Variables|Default|GetxAxis?)
    ;[1 1 1] move x-axis
    (Transformation|SetActorLocation (Math|Vector|MakeVector (+ (* (Math|Trig|Sin(Radians) (* (Utilities|Time|GetTimeSeconds) (Variables|Default|GetSpeed))) (Variables|Default|GetDistance)) _x_2) _y_2 _z_2) false false)
    (else
      ;[1 1 1] move y-axis
      (Transformation|SetActorLocation (Math|Vector|MakeVector _x (+ (* (Math|Trig|Sin(Radians) (* (Utilities|Time|GetTimeSeconds) (Variables|Default|GetSpeed))) (Variables|Default|GetDistance)) _y) _z) false false))))

(fn ConstructionScript
  (Variables|Default|SetStartLocation (Transformation|GetActorLocation)))