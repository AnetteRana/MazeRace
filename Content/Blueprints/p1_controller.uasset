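; Controller Blueprint that spawns and moves all four player pawns for local input, despite its p1 name.
; On BeginPlay it spawns Player1 through Player4 at the first BP_PlayerStart found and stores a reference to each.
; Each Tick it offsets every pawn by its own vertical and horizontal axes times MovementSpeed, without delta-time scaling.
; Movement sets location directly without sweep and pins Z to zero.
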(event EventBeginPlay
  ;[1 1 1] spawn player pawns
  (bind _outactors (Actor|GetAllActorsOfClass "/Game/Blueprints/BP_PlayerStart.BP_PlayerStart_C"))
  (bind _returnvalue (Game|SpawnActorfromClass "/Game/Blueprints/player1.player1_C" (Math|Conversions|ToTransform(Vector) (Transformation|GetActorLocation (Utilities|Array|Get(acopy) _outactors))) "Undefined" 0 0))
  (Variables|Default|Setref_p1 _returnvalue)
  (bind _returnvalue_2 (Game|SpawnActorfromClass "/Game/Blueprints/player2.player2_C" (Math|Conversions|ToTransform(Vector) (Transformation|GetActorLocation (Utilities|Array|Get(acopy) _outactors))) "Undefined" 0 0))
  (Variables|Default|Setref_p2 _returnvalue_2)
  (bind _returnvalue_3 (Game|SpawnActorfromClass "/Game/Blueprints/player3.player3_C" (Math|Conversions|ToTransform(Vector) (Transformation|GetActorLocation (Utilities|Array|Get(acopy) _outactors))) "Undefined" 0 0))
  (Variables|Default|Setref_p3 _returnvalue_3)
  (bind _returnvalue_4 (Game|SpawnActorfromClass "/Game/Blueprints/player4.player4_C" (Math|Conversions|ToTransform(Vector) (Transformation|GetActorLocation (Utilities|Array|Get(acopy) _outactors))) "Undefined" 0 0))
  (Variables|Default|Setref_p4 _returnvalue_4))

(event EventTick
  (params (DeltaSeconds :type Float%20%28single-precision%29))
  (bind _ref_p1 (Variables|Default|Getref_p1))
  (bind _ref_p2 (Variables|Default|Getref_p2))
  (bind _ref_p3 (Variables|Default|Getref_p3))
  (bind _ref_p4 (Variables|Default|Getref_p4))
  (bind _returnvalue (Transformation|GetActorLocation _ref_p1))
  (bind _returnvalue_2 (Transformation|GetActorLocation _ref_p2))
  (bind _returnvalue_3 (Transformation|GetActorLocation _ref_p3))
  (bind _returnvalue_4 (Transformation|GetActorLocation _ref_p4))
  (bind (_x _y) (Math|Vector|BreakVector _returnvalue))
  (bind (_x_2 _y_2) (Math|Vector|BreakVector _returnvalue_4))
  (bind (_x_3 _y_3) (Math|Vector|BreakVector _returnvalue_2))
  (bind (_x_4 _y_4) (Math|Vector|BreakVector _returnvalue_3))
  ;[1 1 1] movement p1
  (Transformation|SetActorLocation _ref_p1 (Math|Vector|MakeVector (+ (* (Variables|Default|GetmovementSpeed) (Input|AxisValues|Getp1_Vertical)) _x) (+ _y (* (Variables|Default|GetmovementSpeed) (Input|AxisValues|Getp1_Horizontal))) 0.0) false false)
  ;[1 1 1] movement p2
  (Transformation|SetActorLocation _ref_p2 (Math|Vector|MakeVector (+ (* (Variables|Default|GetmovementSpeed) (Input|AxisValues|Getp2_Vertical)) _x_3) (+ _y_3 (* (Variables|Default|GetmovementSpeed) (Input|AxisValues|Getp2_Horizontal))) 0.0) false false)
  ;[1 1 1] movement p3
  (Transformation|SetActorLocation _ref_p3 (Math|Vector|MakeVector (+ (* (Variables|Default|GetmovementSpeed) (Input|AxisValues|Getp3_Vertical)) _x_4) (+ _y_4 (* (Variables|Default|GetmovementSpeed) (Input|AxisValues|Getp3_Horizontal))) 0.0) false false)
  ;[1 1 1] movement p4
  (Transformation|SetActorLocation _ref_p4 (Math|Vector|MakeVector (+ (* (Variables|Default|GetmovementSpeed) (Input|AxisValues|Getp4_Vertical)) _x_2) (+ _y_2 (* (Variables|Default|GetmovementSpeed) (Input|AxisValues|Getp4_Horizontal))) 0.0) false false))

(fn ConstructionScript)