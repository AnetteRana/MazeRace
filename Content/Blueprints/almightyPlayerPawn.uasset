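; Player pawn for a maze race game, with its event logic present but disconnected from BeginPlay, Tick and overlap, so none of it runs.
; The unwired logic moves the pawn by P1 input at Z zero and records the BP_PlayerStart location.
; It also switches level through the game mode on touching BP_Goal, otherwise resetting to start.
; SetColor applies a black material to the mesh.
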(event Collision|EventActorBeginOverlap
  (params (OtherActor :type Actor%20Object%20Reference))
  ;[1 1 1] collisions
)

(event EventBeginPlay)

(event EventTick
  (params (DeltaSeconds :type Float%20%28single-precision%29)))

(fn ConstructionScript)

(fn SetColor
  (Rendering|Material|SetMaterial (Variables|Default|GetStaticMesh) 0 "/Game/Materials/MAT_Black.MAT_Black"))